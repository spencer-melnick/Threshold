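; Character Blueprint for Threshold that handles sword setup, melee combat effects and the death sequence.
; BeginPlay equips the Sword; attack events toggle blade trails and spawn a hit effect oriented along the hit velocity.
; Death starts a material dissolve with montage and attached effect, swaps the Sword for a dropped-weapon actor using its mesh, then destroys the character after a delay.
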(event `self.ReceiveTick`
  (params (DeltaSeconds :type "Float (single-precision)"))
  (`KismetSystemLibrary.PrintString` "Hello" true false (struct :`G` 0.66 :`B` 1.0 :`A` 1.0) DeltaSeconds))

(event `self.ReceiveBeginPlay`
  (`self.ChangeActiveWeapon` (`self.Sword`)))

(event `self.OnAttackingActorBP`
  (params (OtherActor :type "Actor Object Reference") (HitResult :type "HitResult Structure") (HitVelocity :type "Vector Structure"))
  (`NiagaraFunctionLibrary.SpawnSystemAtLocation` "/Game/Threshold/Effects/Placeholder/HitEffect_System.HitEffect_System" (`.ImpactPoint` (`GameplayStatics.BreakHitResult` HitResult)) (`KismetMathLibrary.MakeRotFromZ` HitVelocity)))

(event `self.OnAttackDamageStartBP`
  (`ParticleSystemComponent.BeginTrails` (`self.SwordTrail_System`) "BladeTip" "BladeBase" "ETrailWidthMode_FromCentre" 1.0))

(event `self.OnAttackDamageEndBP`
  (`ParticleSystemComponent.EndTrails` (`self.SwordTrail_System`)))

(event `self.OnDeathBP`
  (bind _sword (`self.Sword`))
  (`MaterialDissolveComponent.StartDissolve` (`self.MaterialDissolve`))
  (`AnimInstance.Montage_Play` (`SkeletalMeshComponent.GetAnimInstance` (`self.Mesh`)) "/Game/Threshold/Animations/Placeholder/FullBody/Death_Montage.Death_Montage" 1.0 "MontageLength" 0.0 true)
  (bind _returnvalue (`|SpawnActorFromClass` "/Game/Threshold/Blueprints/Weapons/BP_DroppedWeaponActor.BP_DroppedWeaponActor_C" (`SceneComponent.K2_GetComponentToWorld` (`self.Sword`)) "AdjustIfPossibleButAlwaysSpawn" "OverrideRootScale" null null))
  (`StaticMeshComponent.SetStaticMesh` (`StaticMeshActor.StaticMeshComponent` _returnvalue) (`StaticMeshComponent.StaticMesh` _sword))
  (`ActorComponent.K2_DestroyComponent` _sword)
  (`NiagaraFunctionLibrary.SpawnSystemAttached` "/Game/Threshold/Effects/Placeholder/Dissolve_System.Dissolve_System" (`self.Mesh`) "None" (0.0 0.0 0.0) (struct) "SnapToTargetIncludingScale" true)
  (`KismetSystemLibrary.Delay` 6.0)
  (`self.K2_DestroyActor`))

(fn `UserConstructionScript`)